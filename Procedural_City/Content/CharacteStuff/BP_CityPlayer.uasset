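; BP_CityPlayer is the player's free-moving camera pawn, which creates the road generator UI widget on BeginPlay.
; Enhanced Input actions move it along the camera's forward and right vectors and the actor's up vector.
; A camera lock input gates look rotation and hides the BP_CityController cursor while active, with yaw applied in world space and pitch in local space.
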(event Input|EnhancedActionEvents|EnhancedInputActionIA_Sideways
  (params (ActionValue :type Float%20%28double-precision%29) (ElapsedSeconds :type Float%20%28double-precision%29) (TriggeredSeconds :type Float%20%28double-precision%29) (InputAction :type Input%20Action%20Object%20Reference :default "/Game/CharacteStuff/CityInput/IA_Sideways.IA_Sideways"))
  (Pawn|Input|AddMovementInput (Math|Vector|GetRightVector (Variables|Default|GetCamera)) ActionValue false))

(event Input|EnhancedActionEvents|EnhancedInputActionIA_Forward
  (params (ActionValue :type Float%20%28double-precision%29) (ElapsedSeconds :type Float%20%28double-precision%29) (TriggeredSeconds :type Float%20%28double-precision%29) (InputAction :type Input%20Action%20Object%20Reference :default "/Game/CharacteStuff/CityInput/IA_Forward.IA_Forward"))
  (Pawn|Input|AddMovementInput (Math|Vector|GetForwardVector (Variables|Default|GetCamera)) ActionValue false))

(event Input|EnhancedActionEvents|EnhancedInputActionIA_Up
  (params (ActionValue :type Float%20%28double-precision%29) (ElapsedSeconds :type Float%20%28double-precision%29) (TriggeredSeconds :type Float%20%28double-precision%29) (InputAction :type Input%20Action%20Object%20Reference :default "/Game/CharacteStuff/CityInput/IA_Up.IA_Up"))
  (Pawn|Input|AddMovementInput (Transformation|GetActorUpVector) ActionValue false))

(event Input|EnhancedActionEvents|EnhancedInputActionIA_CameraYaw
  (params (ActionValue :type Float%20%28double-precision%29) (ElapsedSeconds :type Float%20%28double-precision%29) (TriggeredSeconds :type Float%20%28double-precision%29) (InputAction :type Input%20Action%20Object%20Reference :default "/Game/CharacteStuff/CityInput/IA_CameraYaw.IA_CameraYaw"))
  (if (Variables|Default|GetCameraLock)
    (Transformation|AddWorldRotation (Variables|Default|GetCamera) (Math|Rotator|MakeRotator 0.0 0.0 ActionValue) false false)))

(event Input|EnhancedActionEvents|EnhancedInputActionIA_CameraPitch
  (params (ActionValue :type Float%20%28double-precision%29) (ElapsedSeconds :type Float%20%28double-precision%29) (TriggeredSeconds :type Float%20%28double-precision%29) (InputAction :type Input%20Action%20Object%20Reference :default "/Game/CharacteStuff/CityInput/IA_CameraPitch.IA_CameraPitch"))
  (if (Variables|Default|GetCameraLock)
    (Transformation|AddLocalRotation (Variables|Default|GetCamera) (Math|Rotator|MakeRotator 0.0 ActionValue 0.0) false false)))

(event Input|EnhancedActionEvents|EnhancedInputActionIA_CameraLock
  (params (ActionValue :type Boolean) (ElapsedSeconds :type Float%20%28double-precision%29) (TriggeredSeconds :type Float%20%28double-precision%29) (InputAction :type Input%20Action%20Object%20Reference :default "/Game/CharacteStuff/CityInput/IA_CameraLock.IA_CameraLock"))
  (:Started
    (bind _output_get (Variables|Default|SetCameraLock ActionValue :!label _label))
    (bind _asbp_city_controller (Utilities|Casting|CastToBP_CityController (Variables|Default|GetControllerRef)))
    (Variables|/Script/Engine.PlayerController|SetbShowMouseCursor _asbp_city_controller (not _output_get)))
  (:Completed
    (goto _label)))

(event EventBeginPlay
  (bind _returnvalue (UserInterface|CreateWidget "/Game/CharacteStuff/UI/UI_RoadGeneratorUI.UI_RoadGeneratorUI_C"))
  (bind _output_get (Variables|Default|SetVeiewport _returnvalue))
  (UserInterface|Viewport|AddtoViewport _output_get 0)
  (Variables|Default|SetControllerRef (Pawn|GetController)))

(event EventTick
  (params (DeltaSeconds :type Float%20%28single-precision%29)))

(fn ConstructionScript)